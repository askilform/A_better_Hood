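; DamageZone is a trigger volume Blueprint that periodically damages a first-person player character standing inside it.
; Overlapping with BP_FirstPersonCharacter starts a looping one-second timer, which end overlap clears.
; Each tick plays a sound at the character and applies fixed damage.
; If the character's Health then equals exactly zero, it plays a collapse sound and destroys the character.
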(event OnComponentBeginOverlap(DamageZone)
  (params (OverlappedComponent :type Primitive%20Component%20Object%20Reference) (OtherActor :type Actor%20Object%20Reference) (OtherComp :type Primitive%20Component%20Object%20Reference) (OtherBodyIndex :type Integer) (bFromSweep :type Boolean) (SweepResult :type Hit%20Result%20Structure%20%28by%20ref%29))
  (bind _asbp_first_person_character (Utilities|Casting|CastToBP_FirstPersonCharacter OtherActor))
  (Variables|Default|SetAs%20bp%20first%20person _asbp_first_person_character)
  (bind _returnvalue (Utilities|Time|SetTimerbyEvent (delegate Custom|DamagePlayer) 1.0 true))
  (Variables|Default|SetTimerReference _returnvalue))

(event OnComponentEndOverlap(DamageZone)
  (params (OverlappedComponent :type Primitive%20Component%20Object%20Reference) (OtherActor :type Actor%20Object%20Reference) (OtherComp :type Primitive%20Component%20Object%20Reference) (OtherBodyIndex :type Integer))
  (Utilities|Casting|CastToBP_FirstPersonCharacter OtherActor)
  (Utilities|Time|ClearandInvalidateTimerbyHandle (Variables|Default|GetTimerReference)))

(event Custom|DamagePlayer
  (bind _as_bp_first_person (Variables|Default|GetAs%20bp%20first%20person))
  (Audio|PlaySoundatLocation "/Engine/VREditor/Sounds/UI/Camera_Shutter.Camera_Shutter" (Transformation|GetActorLocation _as_bp_first_person) "0, 0, 0" 1.0 1.0 0.0 0 0 0 0)
  (Game|Damage|ApplyDamage (Variables|Default|GetAs%20bp%20first%20person) 1e+01 0 0)
  (if (== (Variables|/Game/FirstPerson/Blueprints/BP_FirstPersonCharacter.BP_FirstPersonCharacter_C|GetHealth _as_bp_first_person) 0.0)
    (Audio|PlaySoundatLocation "/Game/StarterContent/Audio/Collapse01.Collapse01" (Transformation|GetActorLocation _as_bp_first_person) "0, 0, 0" 1.0 1.0 0.0 0 0 0 0)
    (Actor|DestroyActor _as_bp_first_person)))

(fn ConstructionScript)