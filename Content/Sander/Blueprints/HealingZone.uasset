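; Healing zone that restores the first-person player's health while they stand inside its trigger volume.
; Overlap start caches the character and starts a looping one-second timer, which overlap end clears.
; Each tick plays a ping at the player's location, even at full health, and adds a fixed amount of health unless it exactly equals 100, with no clamp.
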(event OnComponentBeginOverlap(HealingZone)
  (params (OverlappedComponent :type Primitive%20Component%20Object%20Reference) (OtherActor :type Actor%20Object%20Reference) (OtherComp :type Primitive%20Component%20Object%20Reference) (OtherBodyIndex :type Integer) (bFromSweep :type Boolean) (SweepResult :type Hit%20Result%20Structure%20%28by%20ref%29))
  (bind _asbp_first_person_character (Utilities|Casting|CastToBP_FirstPersonCharacter OtherActor))
  (Variables|Default|Setas%20bp%20fps _asbp_first_person_character)
  (bind _returnvalue (Utilities|Time|SetTimerbyEvent (delegate Custom|HealPlayer) 1.0 true))
  (Variables|Default|Settimer%20ref _returnvalue))

(event OnComponentEndOverlap(HealingZone)
  (params (OverlappedComponent :type Primitive%20Component%20Object%20Reference) (OtherActor :type Actor%20Object%20Reference) (OtherComp :type Primitive%20Component%20Object%20Reference) (OtherBodyIndex :type Integer))
  (Utilities|Casting|CastToBP_FirstPersonCharacter OtherActor)
  (Utilities|Time|ClearandInvalidateTimerbyHandle (Variables|Default|Gettimer%20ref)))

(event Custom|HealPlayer
  (bind _as_bp_fps (Variables|Default|Getas%20bp%20fps))
  (bind _as_bp_fps_2 (Variables|Default|Getas%20bp%20fps))
  (Audio|PlaySoundatLocation "/Engine/EngineSounds/1kSineTonePing.1kSineTonePing" (Transformation|GetActorLocation _as_bp_fps_2) "0, 0, 0" 1.0 1.0 0.0 0 0 0 0)
  (if (not (== (Variables|/Game/FirstPerson/Blueprints/BP_FirstPersonCharacter.BP_FirstPersonCharacter_C|GetHealth _as_bp_fps_2) 1e+02))
    (Variables|/Game/FirstPerson/Blueprints/BP_FirstPersonCharacter.BP_FirstPersonCharacter_C|SetHealth _as_bp_fps (+ (Variables|/Game/FirstPerson/Blueprints/BP_FirstPersonCharacter.BP_FirstPersonCharacter_C|GetHealth _as_bp_fps) 1e+01))))

(fn ConstructionScript)