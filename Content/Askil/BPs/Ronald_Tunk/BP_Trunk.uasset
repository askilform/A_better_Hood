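; Trunk boss that, once activated, shows its UI, switches to boss music and tracks the player with its rotating sphere.
; It throws projectiles at random intervals, sometimes falling asleep and tilting via timeline to become vulnerable before resuming.
; Taxes actors hitting its Rash while vulnerable deal damage with explosion, shake and voice lines.
; Death resets player health, silences boss music, then explodes and spawns BP_SomeoneDied after a delay.
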(event OnComponentBeginOverlap(Rash)
  (params (OverlappedComponent :type Primitive%20Component%20Object%20Reference) (OtherActor :type Actor%20Object%20Reference) (OtherComp :type Primitive%20Component%20Object%20Reference) (OtherBodyIndex :type Integer) (bFromSweep :type Boolean) (SweepResult :type Hit%20Result%20Structure%20%28by%20ref%29))
  ;[0.15 0.15 0.15 0.5] Damage
  (bind _astaxes (Utilities|Casting|CastToTaxes OtherActor))
  (if (Variables|Default|GetVunerable)
    (CallFunction|SendTaxRef _astaxes)
    (Utilities|FlowControl|Sequence
      (:then_0
        ;;[0.15 0.15 0.15 0.5] Remove damage from health
        (Variables|Default|SetHealth (- (Variables|Default|GetHealth) 15.0)))
      (:then_1
        ;;[0.15 0.15 0.15 0.5] Juice
        (Audio|PlaySound2D "/Game/Askil/BPs/Ronald_Tunk/TrunkDamage.TrunkDamage" 1.0 1.0 0.0 0 0)
        (bind _offset (Timeline|DamageAnim PlayFromStart)
          (:Update
            (Variables|Default|SetOffset_Y_Rotate _offset)
            (bind _asbp_first_person_player_controller (Utilities|Casting|CastToBP_FirstPersonPlayerController (Game|GetPlayerController 0)))
            (Game|Feedback|ClientStartCameraShake _asbp_first_person_player_controller "/Game/Askil/BPs/Ronald_Tunk/BP_CameraShake.BP_CameraShake_C" 1.0 "World" "0, 0, 0")
            (Utilities|FlowControl|Delay 0.5)
            (CallFunction|PlayVoiceLine))))
      (:then_2
        ;;[0.15 0.15 0.15 0.5] Death-Check
        (if (<= (Variables|Default|GetHealth) 0.0)
          (CallFunction|Death))))))

(event Custom|Activate
  ;[0.15 0.15 0.15 0.5] Add HealthBar
  (bind _returnvalue (Actor|GetActorOfClass "/Game/Askil/BPs/BP_Emerg.BP_Emerg_C"))
  (Actor|DestroyActor _returnvalue)
  (Variables|Default|SetActive true)
  (bind _returnvalue_2 (UserInterface|CreateWidget "/Game/Askil/BPs/Ronald_Tunk/Trunk_UI.Trunk_UI_C"))
  (bind _output_get (Variables|Default|SetUI _returnvalue_2))
  (UserInterface|Viewport|AddtoViewport _output_get 0)
  ;[0.15 0.15 0.15 0.5] Turn on bossmusic
  (Audio|Components|Audio|SetVolumeMultiplier (Variables|/Script/Engine.AmbientSound|GetAudioComponent (Variables|Default|GetBossMusic)) 0.15 :!class /Script/Engine.AudioComponent)
  (Audio|Components|Audio|SetVolumeMultiplier (Variables|/Script/Engine.AmbientSound|GetAudioComponent (Variables|Default|GetRegularMusic)) 0.0 :!class /Script/Engine.AudioComponent)
  ;[0.15 0.15 0.15 0.5] Spawn Projectile after random delay
  (Utilities|FlowControl|Delay (Math|Random|RandomFloatinRange 0.0 5.0))
  (if (Variables|Default|GetActive)
    (Game|SpawnActorfromClass "/Game/Askil/BPs/Ronald_Tunk/Projectile.Projectile_C" (Math|Transform|MakeTransform (Transformation|GetWorldLocation (Variables|Default|GetThrowFrom)) "0, 0, 0" "1.000000,1.000000,1.000000") "Undefined" "MultiplyWithRoot" 0 0)
    ;[0.15 0.15 0.15 0.5] Random chance of shooting, or fallingh asleep
    (Math|Integer|CompareInt (Math|Random|RandomIntegerinRange 0 100) 50
      (:>
        (CallFunction|Tired)
        (Audio|PlaySound2D "/Game/Askil/Audio/Snore.Snore" 1.0 1.0 0.0 0 0))
      (:==
        (CallFunction|WaitandShoot :!label _label))
      (:<
        (goto _label)))))

(event Custom|Tired
  ;[0.15 0.15 0.15 0.5] Sleep Cycle
  (if (Variables|Default|GetActive)
    (Utilities|FlowControl|Sequence
      (:then_0
        (Variables|Default|SetVunerable true)
        (bind _0_to__90 (Timeline|RotateToScalp Play)
          (:Update
            (Variables|Default|SetOffset_Y_Rotate _0_to__90))))
      (:then_1
        (Utilities|FlowControl|Delay (Variables|Default|GetTimeVunerable))
        (CallFunction|WaitandShoot)
        (Variables|Default|SetVunerable false)
        (Timeline|RotateToScalp Reverse)))))

(event Custom|WaitAndShoot
  ;[0.15 0.15 0.15 0.5] Spawn Projectile after random delay
  (Utilities|FlowControl|Delay (Math|Random|RandomFloatinRange 0.0 5.0))
  (if (Variables|Default|GetActive)
    (Game|SpawnActorfromClass "/Game/Askil/BPs/Ronald_Tunk/Projectile.Projectile_C" (Math|Transform|MakeTransform (Transformation|GetWorldLocation (Variables|Default|GetThrowFrom)) "0, 0, 0" "1.000000,1.000000,1.000000") "Undefined" "MultiplyWithRoot" 0 0)
    ;[0.15 0.15 0.15 0.5] Random chance of shooting, or fallingh asleep
    (Math|Integer|CompareInt (Math|Random|RandomIntegerinRange 0 100) 50
      (:>
        (CallFunction|Tired)
        (Audio|PlaySound2D "/Game/Askil/Audio/Snore.Snore" 1.0 1.0 0.0 0 0))
      (:==
        (CallFunction|WaitandShoot :!label _label))
      (:<
        (goto _label)))))

(event Custom|Death
  ;[0.15 0.15 0.15 0.5] Death_Sequence
  (Variables|/Game/FirstPerson/Blueprints/BP_FirstPersonCharacter.BP_FirstPersonCharacter_C|SetHealth (Variables|Default|GetPlayer) 1e+02)
  (Variables|Default|SetActive false)
  (Utilities|FlowControl|Sequence
    (:then_0
      ;[0.15 0.15 0.15 0.5] Sleep Cycle
      (CallFunction|WaitandShoot)
      (Variables|Default|SetVunerable false)
      (bind _0_to__90 (Timeline|RotateToScalp Reverse)
        (:Update
          (Variables|Default|SetOffset_Y_Rotate _0_to__90))))
    (:then_1
      (Audio|Components|Audio|SetVolumeMultiplier (Variables|/Script/Engine.AmbientSound|GetAudioComponent (Variables|Default|GetBossMusic)) 0.0 :!class /Script/Engine.AudioComponent))
    (:then_2
      (Utilities|FlowControl|Delay 3.0)
      (Effects|SpawnEmitteratLocation "/Game/StarterContent/Particles/P_Explosion.P_Explosion" (Transformation|GetWorldLocation (Variables|Default|GetSphere)) "0, 0, 0" "10.000000,10.000000,10.000000")
      (Audio|PlaySound2D "/Game/Askil/Audio/Fart2.Fart2" 1.0 1.0 0.0 0 0)
      (Widget|RemovefromParent (Variables|Default|GetUI))
      (Game|SpawnActorfromClass "/Game/Askil/BPs/End/BP_SomeoneDied.BP_SomeoneDied_C" (Math|Transform|MakeTransform "0, 0, 0" "0, 0, 0" "1.000000,1.000000,1.000000") "Undefined" "MultiplyWithRoot" 0 0)
      (Actor|DestroyActor))))

(event Custom|PlayVoiceLine
  ;[0.15 0.15 0.15 0.5] Play Random VoiceLine
  (Audio|PlaySound2D (Utilities|Array|Get(acopy) (Variables|Default|GetVoiceLines) (Math|Random|RandomIntegerinRange 0 (- (Utilities|Array|Length (Variables|Default|GetVoiceLines)) 1))) 1.0 1.0 0.0 0 0))

(event Custom|SendTaxRef
  (params (TaxRef :type Taxes%20Object%20Reference))
  ;[0.15 0.15 0.15 0.5] Damage
  ;;[0.15 0.15 0.15 0.5] Juice
  (Effects|SpawnEmitteratLocation "/Game/StarterContent/Particles/P_Explosion.P_Explosion" (Transformation|GetWorldLocation (Variables|/Script/Engine.Actor|GetRootComponent TaxRef)) "0, 0, 0" "5.000000,5.000000,5.000000"))

(event EventBeginPlay
  ;[0.15 0.15 0.15 0.5] Get Player Reference
  (bind _returnvalue (Actor|GetActorOfClass "/Game/FirstPerson/Blueprints/BP_FirstPersonCharacter.BP_FirstPersonCharacter_C"))
  (Variables|Default|SetPlayer _returnvalue))

(event EventTick
  (params (DeltaSeconds :type Float%20%28single-precision%29))
  (bind _sphere (Variables|Default|GetSphere))
  (bind _player (Variables|Default|GetPlayer))
  (bind _returnvalue (Transformation|GetWorldLocation _sphere))
  (bind _capsulecomponent (Variables|/Script/Engine.Character|GetCapsuleComponent _player))
  (bind _returnvalue_2 (Transformation|GetWorldLocation _capsulecomponent))
  (bind _returnvalue_3 (Math|Rotator|FindLookatRotation _returnvalue _returnvalue_2))
  ;[0.15 0.15 0.15 0.5] Rotate Towards Player Every Frame
  (Transformation|SetWorldRotation _sphere (Math|Rotator|MakeRotator (.roll _returnvalue_3) (+ (.pitch _returnvalue_3) (Variables|Default|GetOffset_Y_Rotate)) (.yaw _returnvalue_3)) false false))

(fn ConstructionScript)