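; BP_Emerg is an actor that steadily drains the player's health until death.
; On BeginPlay it caches the BP_FirstPersonCharacter and starts HealthReduction, a self-calling event that lowers Health by a fixed amount, then repeats after a one-second Delay.
; When Health reaches zero or below, it spawns BP_SomeoneDied and the loop ends.
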(event Custom|HealthReduction
  (bind _player (Variables|Default|GetPlayer))
  ;[0.15 0.15 0.15 0.5] Reduce health every secnod
  (Variables|/Game/FirstPerson/Blueprints/BP_FirstPersonCharacter.BP_FirstPersonCharacter_C|SetHealth _player (- (Variables|/Game/FirstPerson/Blueprints/BP_FirstPersonCharacter.BP_FirstPersonCharacter_C|GetHealth _player) 1.0))
  (if (<= (Variables|/Game/FirstPerson/Blueprints/BP_FirstPersonCharacter.BP_FirstPersonCharacter_C|GetHealth _player) 0.0)
    (Game|SpawnActorfromClass "/Game/Askil/BPs/End/BP_SomeoneDied.BP_SomeoneDied_C" (Math|Transform|MakeTransform "0, 0, 0" "0, 0, 0" "1.000000,1.000000,1.000000") "Undefined" "MultiplyWithRoot" 0 0)
    (else
      (Utilities|FlowControl|Delay 1.0)
      (CallFunction|HealthReduction))))

(event EventBeginPlay
  ;[0.15 0.15 0.15 0.5] Get playerref
  (bind _returnvalue (Actor|GetActorOfClass "/Game/FirstPerson/Blueprints/BP_FirstPersonCharacter.BP_FirstPersonCharacter_C"))
  (Variables|Default|SetPlayer _returnvalue)
  (CallFunction|HealthReduction))

(fn ConstructionScript)