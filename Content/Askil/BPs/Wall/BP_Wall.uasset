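; BP_Wall is a wall actor that blows up once enough "poor guys" are counted against it.
; The AddPoorGuy event adds to a running count and, when it exactly equals ten, latches a Full flag so the sequence fires once.
; After a short delay, it spawns a scaled-up explosion emitter and sound at its root location, then destroys itself.
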(event Custom|AddPoorGuy
  (params (Add :type Integer))
  (bind _defaultsceneroot (Variables|Default|GetDefaultSceneRoot))
  (bind _returnvalue (Transformation|GetWorldLocation _defaultsceneroot))
  (Variables|Default|SetPoorGuys (+ (Variables|Default|GetPoorGuys) Add))
  (if (not (Variables|Default|GetFull))
    (if (== (Variables|Default|GetPoorGuys) 10)
      (Variables|Default|SetFull true)
      (Utilities|FlowControl|Delay 5.0)
      (Effects|SpawnEmitteratLocation "/Game/StarterContent/Particles/P_Explosion.P_Explosion" _returnvalue "0, 0, 0" "50.000000,50.000000,50.000000")
      (Audio|SpawnSoundatLocation "/Game/StarterContent/Audio/Explosion01.Explosion01" _returnvalue "0, 0, 0" 1.0 1.0 0.0 0 0)
      (Actor|DestroyActor))))

(fn ConstructionScript)